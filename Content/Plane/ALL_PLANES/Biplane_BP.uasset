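; Player-flown biplane that flies by applying physics to a Driver component.
; Roll, pitch and yaw inputs add torque, while Tick applies counter-torque damping, constant downward force and a velocity blend toward forward throttle speed.
; Looping timers step the throttle from held inputs and pose PoseableMesh bones, spinning the propeller and deflecting the rudder and left elevator from input.
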(event EventBeginPlay
  (Utilities|Time|SetTimerbyFunctionName 0 "Throttle" 0.05 true)
  (Utilities|Time|SetTimerbyFunctionName 0 "PropRudderElevator" 0.01 true))

(event EventTick
  (params (DeltaSeconds :type Float%20%28single-precision%29))
  (bind _driver (Variables|Default|GetDriver))
  (Class|PrimitiveComponent|AddTorqueinDegrees _driver (/ (Math|Vector|NegateVector (Physics|GetPhysicsAngularVelocityinDegrees (Variables|Default|GetDriver) "None")) "0.500000,0.500000,0.500000") "None" true)
  (Physics|AddForce _driver "0.000000,0.000000,-1500.000000" "None" true)
  (CallFunction|CaculateSpeed))

(event Input|ActionEvents|InputActionThrottleUp
  (params (Key :type Key%20Structure :default "None"))
  (:Pressed
    (Variables|Default|SetThrottle%20Up true))
  (:Released
    (Variables|Default|SetThrottle%20Up false)))

(event Input|ActionEvents|InputActionThrottleDown
  (params (Key :type Key%20Structure :default "None"))
  (:Pressed
    (Variables|Default|SetThrottle%20Down true))
  (:Released
    (Variables|Default|SetThrottle%20Down false)))

(event Input|AxisEvents|InputAxisRoll
  (params (AxisValue :type Float%20%28single-precision%29))
  (Class|PrimitiveComponent|AddTorqueinDegrees (Variables|Default|GetDriver) (Math|Vector|Lerp(Vector) (* (Math|Vector|GetForwardVector (Variables|Default|GetDriver)) (* AxisValue (Variables|Default|GetAir%20Control))) "0, 0, 0" 0.1) "None" true))

(event Input|AxisEvents|InputAxisMoveRIght
  (params (AxisValue :type Float%20%28single-precision%29))
  (Class|PrimitiveComponent|AddTorqueinDegrees (Variables|Default|GetDriver) (Math|Vector|Lerp(Vector) (* (Math|Vector|GetUpVector (Variables|Default|GetDriver)) (* AxisValue (Variables|Default|GetAir%20Control))) "0, 0, 0" 0.1) "None" true))

(event Input|AxisEvents|InputAxisMoveForward
  (params (AxisValue :type Float%20%28single-precision%29))
  (Class|PrimitiveComponent|AddTorqueinDegrees (Variables|Default|GetDriver) (Math|Vector|Lerp(Vector) (* (Math|Vector|GetRightVector (Variables|Default|GetDriver)) (* AxisValue (Variables|Default|GetAir%20Control))) "0, 0, 0" 0.1) "None" true))

(fn ConstructionScript)

(fn Throttle
  (if (Variables|Default|GetThrottle%20Up)
    (bind _result (Math|Integer|IncrementInt (Variables|Default|GetThrottle%20Amount%20))
      (:%20%20
        (bind _output_get (Variables|Default|SetThrottle%20Amount%20 (Math|Integer|Clamp(Integer) _result 0 100)))
        (Development|PrintString (Utilities|String|ToString(Integer) _output_get))))
    (elif (Variables|Default|GetThrottle%20Down)
      (bind _result_2 (Math|Integer|DecrementInt (Variables|Default|GetThrottle%20Amount%20))
        (:%20%20
          (bind _output_get_2 (Variables|Default|SetThrottle%20Amount%20 (Math|Integer|Clamp(Integer) _result_2 0 100)))
          (Development|PrintString (Utilities|String|ToString(Integer) _output_get_2)))))))

(fn CaculateSpeed
  (bind _driver (Variables|Default|GetDriver))
  (bind _returnvalue (Physics|GetPhysicsLinearVelocity _driver "None"))
  (Physics|SetPhysicsLinearVelocity (Variables|Default|GetDriver) (Math|Vector|Lerp(Vector) _returnvalue (* (Math|Vector|GetForwardVector _driver) (Math|Float|Clamp(Float) (Math|Conversions|ToFloat(Integer) (* (Variables|Default|GetThrottle%20Amount%20) 250)) 0.0 2.5e+04)) 0.01) false "None"))

(fn PropRudderElevator
  (bind _poseablemesh (Variables|Default|GetPoseableMesh))
  (bind _poseablemesh_2 (Variables|Default|GetPoseableMesh))
  (bind _poseablemesh_3 (Variables|Default|GetPoseableMesh))
  (bind _returnvalue (Class|PoseableMeshComponent|GetBoneRotationbyName _poseablemesh_3 "Propellor_J" "ComponentSpace"))
  (Components|PoseableMesh|SetBoneRotationbyName _poseablemesh_3 "Propellor_J" (Math|Rotator|MakeRotator (+ (.roll _returnvalue) 2e+01) 0.0 0.0) "ComponentSpace")
  (bind _returnvalue_2 (Class|PoseableMeshComponent|GetBoneRotationbyName _poseablemesh "Rudder_J" "ComponentSpace"))
  (Components|PoseableMesh|SetBoneRotationbyName _poseablemesh "Rudder_J" (Math|Rotator|MakeRotator 0.0 0.0 (Math|Interpolation|FInterpTo (.yaw _returnvalue_2) (* (Input|AxisValues|GetMoveRIght) -35.0) (Utilities|Time|GetWorldDeltaSeconds) 0.0)) "ComponentSpace")
  (bind _returnvalue_3 (Class|PoseableMeshComponent|GetBoneRotationbyName _poseablemesh_2 "Elevator_L_J" "ComponentSpace"))
  (Components|PoseableMesh|SetBoneRotationbyName _poseablemesh_2 "Elevator_L_J" (Math|Rotator|MakeRotator 0.0 (Math|Interpolation|FInterpTo (.yaw _returnvalue_3) (Math|Float|Clamp(Float) (+ (* (Input|AxisValues|GetRoll) -3e+01) (* (Input|AxisValues|GetMoveForward) 3e+01)) -3e+01 3e+01) (Utilities|Time|GetWorldDeltaSeconds) 1e+01) 0.0) "ComponentSpace"))